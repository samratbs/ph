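; BP_Cube_temp is a damage-over-time volume that affects BP_FirstPersonCharacter actors overlapping its Box component.
; Begin overlap calls DOTFunc, which casts to the character, sets its DMGRecieved amount, then calls its DOT and StartDOT.
; End overlap calls EndDOTFunc, which calls EndDOT on the character.
; The damage logic itself lives on the character, and the cube only triggers it.
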(event OnComponentBeginOverlap(Box)
  (params (OverlappedComponent :type Primitive%20Component%20Object%20Reference) (OtherActor :type Actor%20Object%20Reference) (OtherComp :type Primitive%20Component%20Object%20Reference) (OtherBodyIndex :type Integer) (bFromSweep :type Boolean) (SweepResult :type Hit%20Result%20Structure%20%28by%20ref%29))
  (CallFunction|DOTFunc OtherActor))

(event OnComponentEndOverlap(Box)
  (params (OverlappedComponent :type Primitive%20Component%20Object%20Reference) (OtherActor :type Actor%20Object%20Reference) (OtherComp :type Primitive%20Component%20Object%20Reference) (OtherBodyIndex :type Integer))
  (CallFunction|EndDOTFunc OtherActor))

(event EventBeginPlay)

(event Collision|EventActorBeginOverlap
  (params (OtherActor :type Actor%20Object%20Reference)))

(event EventTick
  (params (DeltaSeconds :type Float%20%28single-precision%29)))

(fn ConstructionScript)

(fn DOTFunc
  (params (Object :type Object%20Object%20Reference))
  (bind _asbp_first_person_character (Utilities|Casting|CastToBP_FirstPersonCharacter Object))
  (Utilities|IsValid _asbp_first_person_character
    (:Is%20Valid
      (Variables|/Game/FirstPerson/Blueprints/BP_FirstPersonCharacter.BP_FirstPersonCharacter_C|SetDMG_Recieved _asbp_first_person_character 8.0)
      (Default|DOT _asbp_first_person_character)
      (Default|StartDOT _asbp_first_person_character))))

(fn EndDOTFunc
  (params (Object :type Object%20Object%20Reference))
  (bind _asbp_first_person_character (Utilities|Casting|CastToBP_FirstPersonCharacter Object))
  (Utilities|IsValid _asbp_first_person_character
    (:Is%20Valid
      (Default|EndDOT _asbp_first_person_character))))